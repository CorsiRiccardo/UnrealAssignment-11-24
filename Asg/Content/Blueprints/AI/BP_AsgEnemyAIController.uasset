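; AI controller for BP_AsgEnemy pawns that runs the BT_Enemy behavior tree on BeginPlay.
; Each Tick it measures horizontal (XY) distance to the first player's pawn via CalculateDistance.
; It compares that against the enemy data's acceptable shooting distance and writes the result to the IsInFireRangeKey blackboard bool.
; A PlayerLocationKey blackboard update exists in CalculateDistance but is disconnected and never runs.
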(event EventBeginPlay
  (AI|RunBehaviorTree "/Game/Blueprints/AI/BT_Enemy.BT_Enemy"))

(event EventTick
  (params (DeltaSeconds :type Float%20%28single-precision%29))
  (bind _asbp_asg_enemy (Utilities|Casting|CastToBP_AsgEnemy (Pawn|GetControlledPawn)))
  (bind _distance (CallFunction|CalculateDistance))
  (AI|Components|Blackboard|SetValueasBool (Variables|Default|GetBlackboard) (Variables|Default|GetIsInFireRangeKey) (<= _distance (Variables|/Script/Asg.AsgEnemyDa|GetAcceptableDistanceToShoot (Variables|/Script/Asg.AsgEnemy|GetEnemyData _asbp_asg_enemy)))))

(fn ConstructionScript)

(fn CalculateDistance
  (params (self2 :type Actor%20Object%20Reference))
  (bind _returnvalue (Game|Player|GetPlayerPawn 0))
  (bind _returnvalue_2 (Transformation|GetActorLocation))
  (bind _returnvalue_3 (Transformation|GetActorLocation _returnvalue))
  (return (Math|Float|Absolute(Float) (Math|Vector|Distance2D(Vector) (Math|Vector2D|MakeVector2D (.x _returnvalue_3) (.y _returnvalue_3)) (Math|Vector2D|MakeVector2D (.x _returnvalue_2) (.y _returnvalue_2))))))